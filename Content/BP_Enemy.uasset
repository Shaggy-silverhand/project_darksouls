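; Enemy Blueprint that turns to face the player and plays a light attack montage when the player is in range.
; Tick updates a widget health bar from Health, runs the attack check and yaws the Enemy mesh toward the player while IsLooking is set.
; Lookat and Attack overlap volumes toggle the looking and attack flags.
; A DoOnce gate blocks new attacks until the montage completes.
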(event `self.ReceiveTick`
  (params (DeltaSeconds :type "Float (single-precision)"))
  (bind (_returnvalue_roll _returnvalue_pitch _returnvalue_yaw) (`KismetMathLibrary.BreakRotator` (`KismetMathLibrary.FindLookAtRotation` (`SceneComponent.K2_GetComponentLocation` (`self.enemy`)) (`self.K2_GetActorLocation` (`GameplayStatics.GetPlayerCharacter` 0)))))
  (bind _aswbg_health_bar (cast `/Game/WBG_HealthBar` (`WidgetComponent.GetWidget` (`self.Widget`))))
  (`ProgressBar.SetPercent` (`/Game/WBG_HealthBar.ProgressBar_166` _aswbg_health_bar) (/ (`self.Health`) 100.0))
  (`self.Attacking`)
  (if (`self.IsLooking`)
    (`SceneComponent.K2_SetWorldRotation` (`self.enemy`) (`KismetMathLibrary.MakeRotator` 0.0 0.0 (+ _returnvalue_yaw -90.0)) false false)))

(event `self.Lookat.OnComponentBeginOverlap`
  (params (OverlappedComponent :type "PrimitiveComponent Object Reference") (OtherActor :type "Actor Object Reference") (OtherComp :type "PrimitiveComponent Object Reference") (OtherBodyIndex :type Integer) (bFromSweep :type Boolean) (SweepResult :type "HitResult Structure (by ref)"))
  (set `self.IsLooking` true))

(event `self.Attack.OnComponentBeginOverlap`
  (params (OverlappedComponent :type "PrimitiveComponent Object Reference") (OtherActor :type "Actor Object Reference") (OtherComp :type "PrimitiveComponent Object Reference") (OtherBodyIndex :type Integer) (bFromSweep :type Boolean) (SweepResult :type "HitResult Structure (by ref)"))
  (if (== OtherActor (`GameplayStatics.GetPlayerCharacter` 0))
    (set `self.CanAttack` true)))

(event `Attacking`
  (if (`self.CanAttack`)
    (`/Engine/EditorBlueprintResources/StandardMacros.DoOnce` false :!label _label
      (:`Completed`
        (`|PlayMontage` (`self.enemy`) "/Game/Sword_Animations/montage/LightAttack.LightAttack" 0.4
          (:`OnCompleted`
            (goto _label :!via `Reset`)))))))

(event `self.Lookat.OnComponentEndOverlap`
  (params (OverlappedComponent :type "PrimitiveComponent Object Reference") (OtherActor :type "Actor Object Reference") (OtherComp :type "PrimitiveComponent Object Reference") (OtherBodyIndex :type Integer))
  (set `self.IsLooking` false))

(event `self.Attack.OnComponentEndOverlap`
  (params (OverlappedComponent :type "PrimitiveComponent Object Reference") (OtherActor :type "Actor Object Reference") (OtherComp :type "PrimitiveComponent Object Reference") (OtherBodyIndex :type Integer))
  (set `self.CanAttack` false))

(fn `UserConstructionScript`)